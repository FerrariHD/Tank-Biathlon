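; Player-driven armed race vehicle that stays input-disabled on BeginPlay until the player controller's RaceStart flag, polled on Tick, turns true.
; Axis inputs drive throttle and steering, yaw the turret (Bashnya) and tilt the clamped gun (Pushka2).
; Shell cannon, alternating rocket launcher and alternating twin miniguns spawn projectiles at mesh sockets with sound, shake and particles, gated by flags and delays.
; The M key opens the pause widget and pauses the game.
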(event `self.ReceiveBeginPlay`
  (bind _asmy_player_controller (cast `/Game/VehicleBP/MyPlayerController` (`GameplayStatics.GetPlayerController` 0)))
  (set `self.ControllerReference` _asmy_player_controller)
  (`self.DisableInput` (`self.ControllerReference`)))

(event `self.ReceiveTick`
  (params (DeltaSeconds :type "Float (single-precision)"))
  (bind _controllerreference (`self.ControllerReference`))
  (if (`/Game/VehicleBP/MyPlayerController.RaceStart` _controllerreference)
    (`self.EnableInput` _controllerreference)))

(event `InputAxis|MoveForward`
  (params (AxisValue :type "Float (single-precision)"))
  (`WheeledVehicleMovementComponent.SetThrottleInput` (`self.VehicleMovement`) AxisValue))

(event `InputAxis|MoveRight`
  (params (AxisValue :type "Float (single-precision)"))
  (`WheeledVehicleMovementComponent.SetSteeringInput` (`self.VehicleMovement`) AxisValue))

(event `InputAxis|LookRight`
  (params (AxisValue :type "Float (single-precision)"))
  (`self.AddControllerYawInput` AxisValue))

(event `InputAxis|LookUp`
  (params (AxisValue :type "Float (single-precision)"))
  (bind _relativerotation_roll (`KismetMathLibrary.BreakRotator` (`SceneComponent.RelativeRotation` (`self.Pushka_2`))))
  (bind _relativerotation_roll_2 (`KismetMathLibrary.BreakRotator` (`SceneComponent.RelativeRotation` (`self.Pushka_2`))))
  (`SceneComponent.K2_AddLocalRotation` (`self.Pushka_2`) (`KismetMathLibrary.MakeRotator` (* AxisValue (`self.LookSpeedY`))) false false)
  (if (> _relativerotation_roll 2.0)
    (`SceneComponent.K2_SetRelativeRotation` (`self.Pushka_2`) (`KismetMathLibrary.MakeRotator` 2.0) false false)
    (elif (< _relativerotation_roll_2 -7.0)
      (`SceneComponent.K2_SetRelativeRotation` (`self.Pushka_2`) (`KismetMathLibrary.MakeRotator` -7.0) false false))))

(event `InputAxis|LookRight`
  (params (AxisValue :type "Float (single-precision)"))
  (`SceneComponent.K2_AddLocalRotation` (`self.Bashnya`) (`KismetMathLibrary.MakeRotator` 0.0 0.0 (* AxisValue (`self.LookSpeedX`))) false false))

(event `InputAction|Fire`
  (params (Key :type "Key Structure" :default "AnyKey"))
  (bind _pushka_2 (`self.Pushka_2`))
  (:`Pressed`
    (if (`self.CanFire`)
      (for _array_element (`SceneComponent.GetAllSocketNames` _pushka_2)
        (set `self.CanFire` false)
        (bind _returnvalue (`SceneComponent.GetSocketTransform` _pushka_2 _array_element "RTS_World"))
        (`|SpawnActorFromClass` "/Game/VehicleBP/Shell.Shell_C" _returnvalue "AlwaysSpawn" "OverrideRootScale")
        (bind _location (.location _returnvalue))
        (`GameplayStatics.PlaySoundAtLocation` "/Game/StarterContent/Audio/Explosion01.Explosion01" _location (struct) 1.0 1.0 0.0)
        (`GameplayStatics.PlayWorldCameraShake` "/Game/VehicleBP/ShakeShell.ShakeShell_C" _location 0.0 3000.0)
        (`GameplayStatics.SpawnEmitterAtLocation` "/Game/VehicleBP/P_ExplosionShell.P_ExplosionShell" _location (.rotation _returnvalue))
        (`KismetSystemLibrary.Delay` (`self.FinishDelay`))
        (set `self.CanFire` true)))))

(event `InputAction|RocketFire`
  (params (Key :type "Key Structure" :default "AnyKey"))
  (bind _sm_turret_04 (`self.SM_Turret_04`))
  (bind _leftrightrocket (`self.LeftRightRocket`))
  (bind _returnvalue (`SceneComponent.GetSocketTransform` _sm_turret_04 (`KismetArrayLibrary.Array_Get` (`SceneComponent.GetAllSocketNames` _sm_turret_04) (`KismetMathLibrary.Conv_BoolToInt` _leftrightrocket)) "RTS_World"))
  (bind _location (.location _returnvalue))
  (:`Pressed`
    (if (`self.CanFireRocket`)
      (if _leftrightrocket
        (set `self.LeftRightRocket` false)
        (else
          (set `self.LeftRightRocket` true)))
      (set `self.CanFireRocket` false)
      (`|SpawnActorFromClass` "/Game/VehicleBP/Rocket.Rocket_C" _returnvalue "AlwaysSpawn" "OverrideRootScale")
      (`GameplayStatics.PlaySoundAtLocation` "/Game/StarterContent/Audio/Explosion01.Explosion01" _location (struct) 0.75 0.75 0.0)
      (`GameplayStatics.PlayWorldCameraShake` "/Game/VehicleBP/ShakeRocket.ShakeRocket_C" _location 0.0 3000.0)
      (`GameplayStatics.SpawnEmitterAtLocation` "/Game/VehicleBP/P_ExplosionRocket.P_ExplosionRocket" _location (.rotation _returnvalue))
      (`KismetSystemLibrary.Delay` (`self.FinishDelayRocket`))
      (set `self.CanFireRocket` true))))

(event `InputAction|MiniganFire`
  (params (Key :type "Key Structure" :default "AnyKey"))
  (bind _sm_turret_02 (`self.SM_Turret_02`))
  (bind _sm_turret_01 (`self.SM_Turret_01`))
  (:`Pressed`
    (if (`self.CanFireMinigan`)
      (if (`self.LeftRightMinigan`)
        (set `self.LeftRightMinigan` false)
        (for _array_element (`SceneComponent.GetAllSocketNames` _sm_turret_02)
          (set `self.CanFireMinigan` false)
          (bind _returnvalue (`SceneComponent.GetSocketTransform` _sm_turret_02 _array_element "RTS_World"))
          (`|SpawnActorFromClass` "/Game/VehicleBP/Bullet.Bullet_C" _returnvalue "AlwaysSpawn" "OverrideRootScale")
          (bind _location (.location _returnvalue))
          (`GameplayStatics.PlaySoundAtLocation` "/Game/StarterContent/Audio/Explosion01.Explosion01" _location (struct) 0.5 1.5 0.0)
          (`GameplayStatics.PlayWorldCameraShake` "/Game/VehicleBP/ShakeMinigun.ShakeMinigun_C" _location 0.0 3000.0)
          (`GameplayStatics.SpawnEmitterAtLocation` "/Game/VehicleBP/P_ExplosionMinigun.P_ExplosionMinigun" _location (.rotation _returnvalue))
          (`KismetSystemLibrary.Delay` (`self.FinishDelayMinigan`))
          (set `self.CanFireMinigan` true))
        (else
          (set `self.LeftRightMinigan` true)
          (for _array_element_2 (`SceneComponent.GetAllSocketNames` _sm_turret_01)
            (set `self.CanFireMinigan` false)
            (bind _returnvalue_2 (`SceneComponent.GetSocketTransform` _sm_turret_01 _array_element_2 "RTS_World"))
            (`|SpawnActorFromClass` "/Game/VehicleBP/Bullet.Bullet_C" _returnvalue_2 "AlwaysSpawn" "OverrideRootScale")
            (bind _location_2 (.location _returnvalue_2))
            (`GameplayStatics.PlaySoundAtLocation` "/Game/StarterContent/Audio/Explosion01.Explosion01" _location_2 (struct) 0.5 1.5 0.0)
            (`GameplayStatics.PlayWorldCameraShake` "/Game/VehicleBP/ShakeMinigun.ShakeMinigun_C" _location_2 0.0 3000.0)
            (`GameplayStatics.SpawnEmitterAtLocation` "/Game/VehicleBP/P_ExplosionMinigun.P_ExplosionMinigun" _location_2 (.rotation _returnvalue_2))
            (`KismetSystemLibrary.Delay` (`self.FinishDelayMinigan`))
            (set `self.CanFireMinigan` true)))))))

(event `Key|M`
  (params (Key :type "Key Structure" :default "AnyKey"))
  (bind _returnvalue (`GameplayStatics.GetPlayerController` 0))
  (bind _pausewidgetreference (`self.PauseWidgetReference`))
  (:`Pressed`
    (`/Engine/EditorBlueprintResources/StandardMacros.IsValid` _pausewidgetreference
      (:`Is Valid`
        _)
      (:`Is Not Valid`
        (bind _returnvalue_2 (`|CreateWidget` "/Game/VehicleBP/InGamePauseWidget.InGamePauseWidget_C"))
        (bind _output_get (set `self.PauseWidgetReference` _returnvalue_2))))
    (`WidgetBlueprintLibrary.SetInputMode_UIOnlyEx` _returnvalue _pausewidgetreference)
    (`UserWidget.AddToViewport` _output_get 0)
    (`GameplayStatics.SetGamePaused` true)
    (set `PlayerController.bShowMouseCursor` true _returnvalue)))

(fn `UserConstructionScript`)